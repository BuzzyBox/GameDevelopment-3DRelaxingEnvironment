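; BP_PickUpParent is a base pickup actor that an overlapping actor collects.
; It accepts overlaps from PickupItem_interface implementers other than pickups, sending them item class, icon and stack size through the interface.
; For BP_ThirdPersonCharacter, it also calls JumpCollected, records itself in the GameMode's level save Collected list, prints "Collected" and destroys itself.
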(event Collision|EventActorBeginOverlap
  (params (OtherActor :type Actor%20Object%20Reference))
  (bind _self self)
  (if (Utilities|DoesObjectImplementInterface OtherActor "/Game/Inventory/PickupItem_interface.PickupItem_interface_C")
    (if (not (Utilities|ClassIsChildOf (Utilities|GetClass OtherActor) "BP_PickUpParent_C"))
      (Class|PickupItemInterface|PickupItem(Message) OtherActor (Variables|Default|GetItemClass) (Variables|Default|GetItemIcon) (Variables|Default|GetStackSize))
      (bind _asbp_third_person_character (Utilities|Casting|CastToBP_ThirdPersonCharacter OtherActor))
      (Default|JumpCollected _asbp_third_person_character)
      (Utilities|Array|AddUnique (Variables|/Game/Level/SG_LevelDataObject.SG_LevelDataObject_C|GetCollected (Variables|/Game/ThirdPerson/Blueprints/BP_ThirdPersonGameMode.BP_ThirdPersonGameMode_C|GetLevelSaveObject2 (Variables|/Game/ThirdPerson/Blueprints/BP_ThirdPersonCharacter.BP_ThirdPersonCharacter_C|GetGame%20Mode _asbp_third_person_character))) _self)
      (Development|PrintString "Collected")
      (Actor|DestroyActor _self))))

(fn ConstructionScript)