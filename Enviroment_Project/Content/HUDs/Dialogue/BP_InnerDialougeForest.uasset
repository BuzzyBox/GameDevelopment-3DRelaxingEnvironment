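; BP_InnerDialougeForest steps through inner dialogue lines on screen, apparently for the forest level.
; Each Talk event increments TalkIndex and writes that entry of the Dialouge array into a BP_Dialouge widget, creating it for player 0 if none is valid.
; Once the index passes the last entry, it removes the widget from its parent.
; An unconnected copy of the same logic never runs.
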(event EventTalk
  (Math|Integer|IncrementInt (Variables|Default|GetTalkIndex) ; How much Dialogue is in text
    (:%20%20
      (if (< (Variables|Default|GetTalkIndex) (Utilities|Array|Length (Variables|Default|GetDialouge)))
        ;[1 1 1] Setup UI
        (Variables|Default|GetDialougeUI
          (:then
            _)
          (:else
            (bind _returnvalue (UserInterface|CreateWidget "/Game/HUDs/Dialogue/BP_Dialouge.BP_Dialouge_C" (Game|GetPlayerController 0)))
            (bind _output_get (Variables|Default|SetDialougeUI _returnvalue))
            (UserInterface|Viewport|AddtoViewport _output_get 0)))
        (Rendering|Components|TextRender|SetText (Variables|/Game/HUDs/Dialogue/BP_Dialouge.BP_Dialouge_C|GetTalkText (Variables|Default|GetDialougeUI)) (Utilities|Text|ToText(String) (Utilities|Array|Get(acopy) (Variables|Default|GetDialouge) (Variables|Default|GetTalkIndex))))
        (else
          (Widget|RemovefromParent (Variables|Default|GetDialougeUI)) ; Remove Dialogue in current; level
        )))))

(fn ConstructionScript)