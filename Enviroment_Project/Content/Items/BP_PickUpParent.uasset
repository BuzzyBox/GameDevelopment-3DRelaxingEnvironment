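; BP_PickUpParent is a pickup item actor, named as a parent class, that is collected when a BP_ThirdPersonCharacter overlaps it.
; On overlap it passes its item class, icon and stack size to the character through PickupItem_interface.
; It then records itself in the CollectedItems list of the game mode's level save object and destroys itself.
; The sphere overlap event is empty, and several disconnected leftover nodes remain.
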(event OnComponentBeginOverlap(OverlapSphere)
  (params (OverlappedComponent :type Primitive%20Component%20Object%20Reference) (OtherActor :type Actor%20Object%20Reference) (OtherComp :type Primitive%20Component%20Object%20Reference) (OtherBodyIndex :type Integer) (bFromSweep :type Boolean) (SweepResult :type Hit%20Result%20Structure%20%28by%20ref%29)))

(event Collision|EventActorBeginOverlap
  (params (OtherActor :type Actor%20Object%20Reference))
  (bind _self self)
  (bind _asbp_third_person_character (Utilities|Casting|CastToBP_ThirdPersonCharacter OtherActor))
  (if (Utilities|DoesObjectImplementInterface OtherActor "/Game/Inventory/PickupItem_interface.PickupItem_interface_C")
    (Class|PickupItemInterface|PickupItem(Message) OtherActor (Variables|Default|GetItemClass) (Variables|Default|GetItemIcon) (Variables|Default|GetStackSize))
    (Utilities|Array|AddUnique (Variables|/Game/Savefile/SG_levelDataObject.SG_levelDataObject_C|GetCollectedItems (Variables|/Game/ThirdPerson/Blueprints/BP_ThirdPersonGameMode.BP_ThirdPersonGameMode_C|GetSGLevel%20Save%20Object (Variables|/Game/ThirdPerson/Blueprints/BP_ThirdPersonCharacter.BP_ThirdPersonCharacter_C|GetGame%20Mode _asbp_third_person_character))) _self)
    (Actor|DestroyActor _self)))

(fn ConstructionScript)