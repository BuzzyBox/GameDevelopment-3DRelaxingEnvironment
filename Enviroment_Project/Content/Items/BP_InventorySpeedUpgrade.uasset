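; BP_InventorySpeedUpgrade is an item that grants a speed upgrade to the BP_ThirdPersonCharacter overlapping it.
; On overlap it runs the parent handler, casts to the character, calls its StartSprinting, sets HasSpeed and logs the upgrade.
; Speed changes are left to the character, as the nodes here that edit MaxWalkSpeed are disconnected leftovers that never run.
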(event Collision|EventActorBeginOverlap
  (params (OtherActor :type Actor%20Object%20Reference))
  (|CallParentFunction OtherActor)
  (bind _asbp_third_person_character (Utilities|Casting|CastToBP_ThirdPersonCharacter OtherActor))
  (Default|StartSprinting _asbp_third_person_character)
  (bind _output_get (Variables|/Game/ThirdPerson/Blueprints/BP_ThirdPersonCharacter.BP_ThirdPersonCharacter_C|SetHas%20Speed _asbp_third_person_character true))
  (Utilities|String|LogString "SpeedUpgraded" _output_get))

(fn ConstructionScript)