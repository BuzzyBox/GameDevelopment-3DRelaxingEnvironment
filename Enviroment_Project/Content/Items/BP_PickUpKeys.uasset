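; BP_PickUpKeys is a key pickup that grants the third-person character a key on overlap.
; Overlap calls the parent handler, then sets HasKey on BP_ThirdPersonCharacter and prints it; nothing here removes the pickup.
; Tick spins the static mesh in yaw at SpeedRotation, scaled by delta time.
; A sine-wave bobbing effect is present but disconnected, so it never runs.
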(event EventBeginPlay)

(event Collision|EventActorBeginOverlap
  (params (OtherActor :type Actor%20Object%20Reference))
  (|CallParentFunction OtherActor)
  (bind _asbp_third_person_character (Utilities|Casting|CastToBP_ThirdPersonCharacter OtherActor))
  (bind _output_get (Variables|/Game/ThirdPerson/Blueprints/BP_ThirdPersonCharacter.BP_ThirdPersonCharacter_C|SetHas%20Key? _asbp_third_person_character true))
  (Development|PrintString (Utilities|String|ToString(Boolean) _output_get)))

(event EventTick
  (params (DeltaSeconds :type Float%20%28single-precision%29))
  (Transformation|AddRelativeRotation (Variables|Default|GetStaticMesh) (Math|Rotator|MakeRotator 0.0 0.0 (* DeltaSeconds (Variables|Default|GetSpeed%20Rotation))) false false))

(fn ConstructionScript
  (|CallParentFunction))