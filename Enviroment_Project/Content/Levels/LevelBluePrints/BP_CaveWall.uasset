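; BP_CaveWall is a cave wall actor that shows player monologue when the third-person character enters its trigger box.
; Box overlap creates a PlayerMonologue widget and removes it on exit.
; EventDialogueOccurs disables movement and advances the widget's row through NPCText, restoring walking after the last line.
; A DoOnce, reset by ResetDialogue, gates each advance, while CheckSpeaking always returns false.
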(event OnComponentBeginOverlap(Box)
  (params (OverlappedComponent :type Primitive%20Component%20Object%20Reference) (OtherActor :type Actor%20Object%20Reference) (OtherComp :type Primitive%20Component%20Object%20Reference) (OtherBodyIndex :type Integer) (bFromSweep :type Boolean) (SweepResult :type Hit%20Result%20Structure%20%28by%20ref%29))
  (Utilities|Casting|CastToBP_ThirdPersonCharacter OtherActor)
  (bind _returnvalue (UserInterface|CreateWidget "/Game/Blueprints/PlayerMonologue.PlayerMonologue_C"))
  (bind _output_get (Variables|Default|SetDialogue _returnvalue))
  (UserInterface|Viewport|AddtoViewport _output_get 0))

(event OnComponentEndOverlap(Box)
  (params (OverlappedComponent :type Primitive%20Component%20Object%20Reference) (OtherActor :type Actor%20Object%20Reference) (OtherComp :type Primitive%20Component%20Object%20Reference) (OtherBodyIndex :type Integer))
  (bind _dialogue (Variables|Default|GetDialogue))
  (Utilities|Casting|CastToBP_ThirdPersonCharacter OtherActor)
  (Utilities|IsValid _dialogue
    (:Is%20Valid
      (Widget|RemovefromParent _dialogue))))

(event Custom|ResetDialogue
  (Utilities|FlowControl|DoOnce false) ; enters at Reset
)

(event EventEventDialogueOccurs
  (bind _asbp_third_person_character (Utilities|Casting|CastToBP_ThirdPersonCharacter (Game|GetPlayerCharacter 0)))
  (Pawn|Components|CharacterMovement|SetMovementMode (Variables|/Script/Engine.Character|GetCharacterMovement _asbp_third_person_character) "MOVE_None" 0)
  (Utilities|FlowControl|DoOnce false
    (:Completed
      (Variables|/Game/Blueprints/PlayerMonologue.PlayerMonologue_C|SetText (Variables|Default|GetDialogue) (Variables|Default|GetNPCText))
      (Widget|SetVisibility (Variables|/Game/Blueprints/PlayerMonologue.PlayerMonologue_C|GetSpeechBubble (Variables|Default|GetDialogue)) "Visible")
      (if (> (+ (Variables|/Game/Blueprints/PlayerMonologue.PlayerMonologue_C|GetTextRow (Variables|Default|GetDialogue)) 1) (- (Utilities|Array|Length (Variables|Default|GetNPCText)) 1))
        (Widget|RemovefromParent (Variables|Default|GetDialogue))
        (CallFunction|ResetDialogue)
        (bind _asbp_third_person_character_2 (Utilities|Casting|CastToBP_ThirdPersonCharacter (Game|GetPlayerCharacter 0)))
        (Pawn|Components|CharacterMovement|SetMovementMode (Variables|/Script/Engine.Character|GetCharacterMovement _asbp_third_person_character_2) "MOVE_Walking" 0)
        (else
          (Variables|/Game/Blueprints/PlayerMonologue.PlayerMonologue_C|SetTextRow (Variables|Default|GetDialogue) (+ (Variables|/Game/Blueprints/PlayerMonologue.PlayerMonologue_C|GetTextRow (Variables|Default|GetDialogue)) 1))
          (CallFunction|ResetDialogue))))))

(fn ConstructionScript)

(fn CheckSpeaking
  (return false))