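; Spline-driven fence layout tool that builds a run of spline meshes along its Spline component in the construction script.
; The spline length divided by SectionLength sets the segment count, with separate mesh component templates for first, middle and last pieces.
; Each piece spans one SectionLength along X with query and physics collision.
; Tangents come from spline locations, rather than spline tangents, clamped to SectionLength.
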(event EventBeginPlay)

(event Collision|EventActorBeginOverlap
  (params (OtherActor :type Actor%20Object%20Reference)))

(event EventTick
  (params (DeltaSeconds :type Float%20%28single-precision%29)))

(fn ConstructionScript
  (bind _spline (Variables|Default|GetSpline))
  (bind _spline_2 (Variables|Default|GetSpline))
  (bind _spline_3 (Variables|Default|GetSpline))
  (bind _sectionlength (Variables|Default|GetSectionLength))
  (bind _sectionlength_2 (Variables|Default|GetSectionLength))
  (bind _returnvalue (Spline|GetSplineLength _spline_3))
  (bind _returnvalue_2 (/ _returnvalue _sectionlength))
  (bind _returnvalue_3 (Math|Float|Truncate _returnvalue_2))
  (bind _returnvalue_4 (- _returnvalue_3 0))
  (for _index (range 0 _returnvalue_4)
    (if (== _index 0)
      (bind _returnvalue_5 (AddComponent|AddSplineMeshComponent false))
      (Variables|Default|SetInstance _returnvalue_5)
      (elif (== _index _returnvalue_4)
        (bind _returnvalue_6 (AddComponent|AddSplineMeshComponent false))
        (Variables|Default|SetInstance _returnvalue_6)
        (else
          (bind _returnvalue_7 (AddComponent|AddSplineMeshComponent false))
          (Variables|Default|SetInstance _returnvalue_7))))
    (SplineMesh|SetForwardAxis (Variables|Default|GetInstance) "X" true)
    (SplineMesh|SetStartandEnd (Variables|Default|GetInstance) (Spline|GetLocationatDistanceAlongSpline _spline (* _index _sectionlength_2) "Local") (Math|Vector|ClampVectorSize (Spline|GetLocationatDistanceAlongSpline _spline (* _index _sectionlength_2) "Local") 0.0 (Variables|Default|GetSectionLength)) (Spline|GetLocationatDistanceAlongSpline _spline_2 (* (+ _index 1) _sectionlength_2) "Local") (Math|Vector|ClampVectorSize (Spline|GetLocationatDistanceAlongSpline _spline_2 (* (+ _index 1) _sectionlength_2) "Local") 0.0 (Variables|Default|GetSectionLength)) true :!class /Script/Engine.SplineMeshComponent)
    (Collision|SetCollisionEnabled (Variables|Default|GetInstance) "QueryAndPhysics")))