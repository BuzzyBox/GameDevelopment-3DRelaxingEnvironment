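; A test dialogue actor that shows a PlayerMonologue widget while the third-person character overlaps its DialogueHitbox and removes it on exit.
; EventDialogueOccurs passes the NPCText lines to the widget, shows the speech bubble, and advances TextRow, removing the widget once the last row is reached.
; A DoOnce guards each step and is immediately reset through ResetDialogue.
; A debug print remains, and CheckSpeaking is a stub returning false.
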(event OnComponentBeginOverlap(DialogueHitbox)
  (params (OverlappedComponent :type Primitive%20Component%20Object%20Reference) (OtherActor :type Actor%20Object%20Reference) (OtherComp :type Primitive%20Component%20Object%20Reference) (OtherBodyIndex :type Integer) (bFromSweep :type Boolean) (SweepResult :type Hit%20Result%20Structure%20%28by%20ref%29))
  (Utilities|Casting|CastToBP_ThirdPersonCharacter OtherActor)
  (bind _returnvalue (UserInterface|CreateWidget "/Game/Blueprints/PlayerMonologue.PlayerMonologue_C"))
  (bind _output_get (Variables|Default|SetDialogueUI _returnvalue))
  (UserInterface|Viewport|AddtoViewport _output_get 0))

(event OnComponentEndOverlap(DialogueHitbox)
  (params (OverlappedComponent :type Primitive%20Component%20Object%20Reference) (OtherActor :type Actor%20Object%20Reference) (OtherComp :type Primitive%20Component%20Object%20Reference) (OtherBodyIndex :type Integer))
  (bind _dialogueui (Variables|Default|GetDialogueUI))
  (Utilities|Casting|CastToBP_ThirdPersonCharacter OtherActor)
  (Utilities|IsValid _dialogueui
    (:Is%20Valid
      (Widget|RemovefromParent _dialogueui))))

(event Custom|ResetDialogue
  (Utilities|FlowControl|DoOnce false) ; enters at Reset
)

(event EventEventDialogueOccurs
  (Development|PrintString "Test")
  (Utilities|FlowControl|DoOnce false
    (:Completed
      (Variables|/Game/Blueprints/PlayerMonologue.PlayerMonologue_C|SetText (Variables|Default|GetDialogueUI) (Variables|Default|GetNPCText))
      (Widget|SetVisibility (Variables|/Game/Blueprints/PlayerMonologue.PlayerMonologue_C|GetSpeechBubble (Variables|Default|GetDialogueUI)) "Visible")
      (if (> (+ (Variables|/Game/Blueprints/PlayerMonologue.PlayerMonologue_C|GetTextRow (Variables|Default|GetDialogueUI)) 1) (- (Utilities|Array|Length (Variables|Default|GetNPCText)) 1))
        (Widget|RemovefromParent (Variables|Default|GetDialogueUI))
        (CallFunction|ResetDialogue)
        (else
          (Variables|/Game/Blueprints/PlayerMonologue.PlayerMonologue_C|SetTextRow (Variables|Default|GetDialogueUI) (+ (Variables|/Game/Blueprints/PlayerMonologue.PlayerMonologue_C|GetTextRow (Variables|Default|GetDialogueUI)) 1))
          (CallFunction|ResetDialogue))))))

(fn ConstructionScript)

(fn CheckSpeaking
  (return false))