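; A test dialogue trigger that shows a PlayerMonologue widget while the third-person character overlaps its box and removes it on exit.
; EventDialogueOccurs passes the NPCText lines to the widget, reveals its speech bubble and advances TextRow, removing the widget once no next row remains.
; A DoOnce gate guards each advance and is reset afterward through ResetDialogue.
; CheckSpeaking is a stub returning false.
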(event OnComponentBeginOverlap(Box)
  (params (OverlappedComponent :type Primitive%20Component%20Object%20Reference) (OtherActor :type Actor%20Object%20Reference) (OtherComp :type Primitive%20Component%20Object%20Reference) (OtherBodyIndex :type Integer) (bFromSweep :type Boolean) (SweepResult :type Hit%20Result%20Structure%20%28by%20ref%29))
  (Utilities|Casting|CastToBP_ThirdPersonCharacter OtherActor)
  (bind _returnvalue (UserInterface|CreateWidget "/Game/Blueprints/PlayerMonologue.PlayerMonologue_C"))
  (bind _output_get (Variables|Default|SetDialogue%20UI _returnvalue))
  (UserInterface|Viewport|AddtoViewport _output_get 0))

(event OnComponentEndOverlap(Box)
  (params (OverlappedComponent :type Primitive%20Component%20Object%20Reference) (OtherActor :type Actor%20Object%20Reference) (OtherComp :type Primitive%20Component%20Object%20Reference) (OtherBodyIndex :type Integer))
  (bind _dialogue_ui (Variables|Default|GetDialogue%20UI))
  (Utilities|Casting|CastToBP_ThirdPersonCharacter OtherActor)
  (Utilities|IsValid _dialogue_ui
    (:Is%20Valid
      (Widget|RemovefromParent _dialogue_ui))))

(event Custom|ResetDialogue
  (Utilities|FlowControl|DoOnce false) ; enters at Reset
)

(event EventEventDialogueOccurs
  (Utilities|FlowControl|DoOnce false
    (:Completed
      (Variables|/Game/Blueprints/PlayerMonologue.PlayerMonologue_C|SetText (Variables|Default|GetDialogue%20UI) (Variables|Default|GetNPCText))
      (Widget|SetVisibility (Variables|/Game/Blueprints/PlayerMonologue.PlayerMonologue_C|GetSpeechBubble (Variables|Default|GetDialogue%20UI)) "Visible")
      (if (> (+ (Variables|/Game/Blueprints/PlayerMonologue.PlayerMonologue_C|GetTextRow (Variables|Default|GetDialogue%20UI)) 1) (- (Utilities|Array|Length (Variables|Default|GetNPCText)) 1))
        (Widget|RemovefromParent (Variables|Default|GetDialogue%20UI))
        (CallFunction|ResetDialogue)
        (else
          (Variables|/Game/Blueprints/PlayerMonologue.PlayerMonologue_C|SetTextRow (Variables|Default|GetDialogue%20UI) (+ (Variables|/Game/Blueprints/PlayerMonologue.PlayerMonologue_C|GetTextRow (Variables|Default|GetDialogue%20UI)) 1))
          (CallFunction|ResetDialogue))))))

(fn ConstructionScript)

(fn CheckSpeaking
  (return false))