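; Dialogue Blueprint that feeds lines from its Dialogue array to the player character for display.
; The Speaking event first checks CheckSpeakingMessage on the player, and only when that is false passes the current entry to SpeakingMessage.
; It then increments CurrentDialogue but immediately resets it to zero, since the end-of-array comparison is not wired into the always-true branch.
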(event Custom|Speaking
  (bind _bespeaking (Class|PlayerVPI|CheckSpeaking(Message) (Game|GetPlayerCharacter 0)))
  (if (not _bespeaking)
    (Class|PlayerVPI|Speaking(Message) (Game|GetPlayerCharacter 0) (Utilities|Array|Get(acopy) (Variables|Default|GetDialogue) (Variables|Default|GetCurrentDialogue)))
    (bind _result (Math|Integer|IncrementInt (Variables|Default|GetCurrentDialogue))
      (:%20%20
        (if true
          (Variables|Default|SetCurrentDialogue 0))))))