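; Master Blueprint for floating objects in MagicStonesIsland, animating a configurable static mesh.
; The construction script applies the Mesh variable to the StaticMesh component.
; On BeginPlay, the Floating timeline starts at a random play rate, so instances move at different speeds.
; Its single track scales the X, Y and Z variables, which drive both relative location and rotation (roll, pitch, yaw).
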(event EventBeginPlay
  (Components|Timeline|SetPlayRate (Variables|Default|GetFloating) (Math|Random|RandomFloatinRange 0.1 1.0))
  (bind _newtrack_0 (Timeline|Floating Play)
    (:Update
      (Transformation|SetRelativeLocationAndRotation (Variables|Default|GetStaticMesh) (Math|Vector|MakeVector (* _newtrack_0 (Variables|Default|GetX)) (* _newtrack_0 (Variables|Default|GetY)) (* _newtrack_0 (Variables|Default|GetZ))) (Math|Rotator|MakeRotator (* _newtrack_0 (Variables|Default|GetX)) (* _newtrack_0 (Variables|Default|GetY)) (* _newtrack_0 (Variables|Default|GetZ))) false false))))

(fn ConstructionScript
  (Components|StaticMesh|SetStaticMesh (Variables|Default|GetStaticMesh) (Variables|Default|GetMesh)))