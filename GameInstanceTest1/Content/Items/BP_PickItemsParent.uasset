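; Parent Blueprint for pickup items that hand themselves to the player when touched.
; An overlap sphere checks that the other actor is the player, implements PickUpItems_Interface and is not itself a pickup.
; It sends item class, icon and stack size through the interface, then destroys itself once the BP_ThirdPersonCharacter cast succeeds.
; PickupItemsData is a stub returning zero stack amounts.
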(event OnComponentBeginOverlap(OverlapSphare)
  (params (OverlappedComponent :type Primitive%20Component%20Object%20Reference) (OtherActor :type Actor%20Object%20Reference) (OtherComp :type Primitive%20Component%20Object%20Reference) (OtherBodyIndex :type Integer) (bFromSweep :type Boolean) (SweepResult :type Hit%20Result%20Structure%20%28by%20ref%29))
  (if (== OtherActor (Game|GetPlayerCharacter 0))
    (if (Utilities|DoesObjectImplementInterface OtherActor "/Game/Items/PickUpItems_Interface.PickUpItems_Interface_C")
      (if (not (Utilities|ClassIsChildOf (Utilities|GetClass OtherActor) "BP_PickItemsParent_C"))
        (Class|PickUpItemsInterface|PickupItems(Message) OtherActor (Variables|Default|GetItemClass) (Variables|Default|GetItemIcon) (Variables|Default|GetStackSize))
        (bind _asbp_third_person_character (Utilities|Casting|CastToBP_ThirdPersonCharacter (Game|GetPlayerCharacter 0)))
        (Variables|Default|SetCharacterItemPickup _asbp_third_person_character)
        (Actor|DestroyActor self)))))

(event Collision|EventActorBeginOverlap
  (params (OtherActor :type Actor%20Object%20Reference)))

(fn ConstructionScript)

(fn PickupItemsData
  (return 0 0 0))