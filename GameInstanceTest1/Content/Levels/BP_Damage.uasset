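; BP_Damage is a level actor that changes the player's health when the player overlaps its DamageCollision component.
; On BeginPlay it casts the player character to BP_ThirdPersonCharacter and caches the reference.
; Each player overlap adds HealthVariable to Health, so damage depends on a negative value, then calls CallUpdateHealth with the new total.
; The change is applied directly, without Unreal's damage system or clamping in this Blueprint.
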(event OnComponentBeginOverlap(DamageCollision)
  (params (OverlappedComponent :type Primitive%20Component%20Object%20Reference) (OtherActor :type Actor%20Object%20Reference) (OtherComp :type Primitive%20Component%20Object%20Reference) (OtherBodyIndex :type Integer) (bFromSweep :type Boolean) (SweepResult :type Hit%20Result%20Structure%20%28by%20ref%29))
  (bind _ascharacter (Variables|Default|GetAsCharacter))
  (if (== OtherActor (Game|GetPlayerCharacter 0))
    (bind _output_get (Variables|/Game/ThirdPerson/Blueprints/BP_ThirdPersonCharacter.BP_ThirdPersonCharacter_C|SetHealth _ascharacter (+ (Variables|/Game/ThirdPerson/Blueprints/BP_ThirdPersonCharacter.BP_ThirdPersonCharacter_C|GetHealth _ascharacter) (Variables|Default|GetHealthVariable))))
    (Default|CallUpdateHealth _ascharacter _output_get)))

(event EventBeginPlay
  (bind _asbp_third_person_character (Utilities|Casting|CastToBP_ThirdPersonCharacter (Game|GetPlayerCharacter 0)))
  (Variables|Default|SetAsCharacter _asbp_third_person_character))

(fn ConstructionScript)